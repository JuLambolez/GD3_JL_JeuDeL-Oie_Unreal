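; BP_Tile is a single board square for a Game of the Goose (Jeu de l'Oie) board.
; On BeginPlay it writes its ID onto the TileNumber text.
; It then switches on TileType (Normal, Forward, Backward or Mini Game) to give the Cube mesh the matching material.
; The Blueprint only handles display: it holds no movement or mini-game logic, and its construction script is empty.
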(event EventBeginPlay
  (bind _cube (Variables|Default|GetCube))
  (bind _cube_2 (Variables|Default|GetCube))
  ;[0.15 0.15 0.15 0.5] Récupère l'ID de la case, et l'affiche sur la case
  (Rendering|Components|TextRender|SetText (Variables|Default|GetTileNumber) (Utilities|Text|ToText(Integer) (Variables|Default|GetID)))
  ;[0.15 0.15 0.15 0.5] Set le material de la Tile en fonction de son type
  (switch Utilities|FlowControl|Switch|SwitchonE_TileType (Variables|Default|GetTileType)
    (:NewEnumerator0
      (Rendering|Material|SetMaterial _cube_2 0 "/Game/JeuDeL-Oie/Board/Cases/Materials/M_TileClassic.M_TileClassic"))
    (:NewEnumerator1
      (Rendering|Material|SetMaterial _cube_2 0 "/Game/JeuDeL-Oie/Board/Cases/Materials/M_TileForward.M_TileForward"))
    (:NewEnumerator2
      (Rendering|Material|SetMaterial _cube 0 "/Game/JeuDeL-Oie/Board/Cases/Materials/M_TileBackwards.M_TileBackwards"))
    (:NewEnumerator3
      (Rendering|Material|SetMaterial _cube 0 "/Game/JeuDeL-Oie/Board/Cases/Materials/M_TileMiniGame.M_TileMiniGame"))))

(fn ConstructionScript)