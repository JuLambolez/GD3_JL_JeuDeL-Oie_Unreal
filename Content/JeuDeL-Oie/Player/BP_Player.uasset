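; Player pawn for a Game of the Goose board game, starting on the first tile of BP_Board.
; Holding Space spins a 3D die; releasing rolls 1 to 6 while timelines slow and raise the die, then pop up the result text.
; ComputePath builds MovePath with a bounce-back at the last tile.
; MoveNextStep recursively counts down eased moves, though these always target tile 0, and its end branch always prints victory.
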(event Custom|MoveNextStep
  (if (< (Variables|Default|GetStepCounter) (Utilities|Array|Length (Variables|Default|GetMovePath)))
    (Components|MoveComponentTo (Variables|Default|GetDefaultSceneRoot) (+ (Transformation|GetActorLocation (Utilities|Array|Get(acopy) (Variables|/Game/JeuDeL-Oie/Board/BP_Board.BP_Board_C|GetTiles (Variables|Default|GetBoard)))) (Variables|Default|GetPlayerOffset)) "0, 0, 0" true true (Variables|Default|GetStepDuration) false)
    (Variables|Default|SetCurrentIndex 0)
    (Variables|Default|SetRemainingSteps (- (Variables|Default|GetRemainingSteps) 1))
    (if (> (Variables|Default|GetRemainingSteps) 0)
      (Rendering|Components|TextRender|SetText (Variables|Default|GetResultext) (Utilities|Text|ToText(Integer) (Variables|Default|GetRemainingSteps)))
      (Variables|Default|SetStepCounter (+ (Variables|Default|GetStepCounter) 1))
      (CallFunction|MoveNextStep))
    (else
      (Rendering|SetVisibility (Variables|Default|GetResultext) false false)
      (if true
        (Development|PrintString "VICTOIRE")
        (else
          (Variables|Default|SetbBusy false))))))

(event EventBeginPlay
  (Variables|Default|SetStarLocation (Variables|/Script/Engine.SceneComponent|GetRelativeLocation (Variables|Default|GetDice)))
  (bind _returnvalue (Actor|GetActorOfClass "/Game/JeuDeL-Oie/Board/BP_Board.BP_Board_C"))
  (bind _output_get (Variables|Default|SetBoard _returnvalue))
  (Transformation|SetActorLocation (+ (Variables|Default|GetPlayerOffset) (Transformation|GetActorLocation (Utilities|Array|Get(acopy) (Variables|/Game/JeuDeL-Oie/Board/BP_Board.BP_Board_C|GetTiles _output_get)))) false false)
  (Variables|Default|SetCurrentIndex 0))

(event EventTick
  (params (DeltaSeconds :type Float%20%28single-precision%29))
  ;[0.15 0.15 0.15 0.5] Animation de rotation du dé qui se fait
  (if (Variables|Default|GetbRolling)
    (Transformation|AddLocalRotation (Variables|Default|GetDice) (* (* (Variables|Default|GetRotSpeed) DeltaSeconds) (Variables|Default|GetSpeedMultiplayer)) false false)))

(event Input|KeyboardEvents|SpaceBar
  (params (Key :type Key%20Structure :default "None"))
  (bind _resultext (Variables|Default|GetResultext))
  (bind _dice (Variables|Default|GetDice))
  (:Pressed
    (if (not (Variables|Default|GetbBusy))
      (Rendering|SetVisibility (Variables|Default|GetResultext) false false)
      (Rendering|SetVisibility _dice true false)
      (Transformation|SetRelativeLocation _dice (Variables|Default|GetStarLocation) false false)
      (Variables|Default|SetbRolling true)
      (Variables|Default|SetSpeedMultiplayer 1.0)))
  (:Released
    (if (Variables|Default|GetbRolling)
      (Variables|Default|SetbBusy true)
      (bind _output_get (Variables|Default|SetResult (Math|Random|RandomIntegerinRange 1 6)))
      (CallFunction|ComputePath _output_get)
      (Components|Timeline|SetPlayRate (Variables|Default|GetTL_DiceRelease) (/ 1.0 (Variables|Default|GetSlowDownDuration)))
      (bind _alpha (Timeline|TL_DiceRelease PlayFromStart)
        (:Update
          (Variables|Default|SetSpeedMultiplayer (- 1.0 _alpha))
          (Transformation|SetRelativeLocation (Variables|Default|GetDice) (Math|Vector|Lerp(Vector) (Variables|Default|GetStarLocation) (+ (Variables|Default|GetStarLocation) (Math|Vector|MakeVector 0.0 0.0 (Variables|Default|GetRiseHeight))) _alpha) false false))
        (:Finished
          (Variables|Default|SetbRolling false)
          (Rendering|SetVisibility (Variables|Default|GetDice) false false)
          (Rendering|Components|TextRender|SetText _resultext (Utilities|Text|ToText(Integer) (Variables|Default|GetResult)))
          (Transformation|SetRelativeScale3D _resultext "0, 0, 0")
          (Rendering|SetVisibility _resultext true false)
          (Components|Timeline|SetPlayRate (Variables|Default|GetTL_TextPop) (/ 1.0 (Variables|Default|GetPopDuration)))
          (bind _scale (Timeline|TL_TextPop PlayFromStart)
            (:Update
              (Transformation|SetRelativeScale3D (Variables|Default|GetResultext) (Math|Vector|MakeVector _scale _scale _scale)))
            (:Finished
              (Utilities|FlowControl|Delay 0.5)
              (Variables|Default|SetStepCounter 0)
              (Variables|Default|SetRemainingSteps (Variables|Default|GetResult))
              (CallFunction|MoveNextStep))))))))

(fn ConstructionScript)

(fn ComputePath
  (params (Roll :type Integer))
  (Utilities|Array|Clear (Variables|Default|GetMovePath))
  (LocalVariables|SetSimIndex (Variables|Default|GetCurrentIndex))
  (LocalVariables|SetSimDir 1)
  (LocalVariables|SetLast (- (Utilities|Array|Length (Variables|/Game/JeuDeL-Oie/Board/BP_Board.BP_Board_C|GetTiles (Variables|Default|GetBoard))) 1))
  (for _index (range 0 (- Roll 1))
    (if (>= (LocalVariables|GetSimIndex) (LocalVariables|GetLast))
      (LocalVariables|SetSimDir -1)
      (LocalVariables|SetSimIndex (+ (LocalVariables|GetSimIndex) (LocalVariables|GetSimDir)))
      (Utilities|Array|Add (Variables|Default|GetMovePath) (LocalVariables|GetSimIndex)))))